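; Player controller that creates the sample HUD and switches the view between Walk, Turn and Orbit cameras with cubic blends.
; While the left mouse is dragged, Tick applies the offset from the press point to turn or orbit rotation.
; Orbit initializes lazily from its target on first drag, and the wheel changes its distance.
; FindScene, FindPhoto and FindMovie trigger numbered scene, photo and movie actors, with FindScene also updating the HUD label.
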(event Custom|CreateHUD
  (Utilities|IsValid (Variables|Default|GetSampleWidget)
    (:Is%20Not%20Valid
      (bind _returnvalue (UserInterface|CreateWidget "/Game/Sample0216/UI/SampleWidgetBP.SampleWidgetBP_C" self))
      (bind _output_get (Variables|Default|SetSampleWidget _returnvalue))
      (UserInterface|Viewport|AddtoViewport _output_get 0)
      (bind _returnvalue_2 (UserInterface|CreateWidget "/Game/Sample0216/UI/MediaWidgetBP.MediaWidgetBP_C" self))
      (UserInterface|Viewport|AddtoViewport (stale _output_get) 0))))

(event Custom|SetUp
  (Default|SetSceneName (Variables|Default|GetSampleWidget) (Variables|Default|GetCurrentCameraName)))

(event Custom|ChangeCameraMode
  (params (CameraMode :type Integer))
  (CallFunction|ChangeCamera CameraMode)
  (Default|SetSceneName (Variables|Default|GetSampleWidget) (Variables|Default|GetCurrentCameraName)))

(event Custom|FindMovie
  (params (Number :type Integer) (Show :type Boolean))
  (bind _outactors (Actor|GetAllActorsOfClass "/Game/Sample0216/Blueprints/MoviePlayBP.MoviePlayBP_C"))
  (for _array_element _outactors
    (if (== (Variables|/Game/Sample0216/Blueprints/MoviePlayBP.MoviePlayBP_C|GetNumber _array_element) Number) ; SceneNumberと同じBPを探す
      (Default|PlayMovie _array_element Show))))

(event Custom|MovieUI
  (params (Show :type Boolean))
  (bind _returnvalue (UserInterface|CreateWidget "/Game/Sample0216/UI/MediaWidgetBP.MediaWidgetBP_C" self))
  (UserInterface|Viewport|AddtoViewport _returnvalue 0))

(event Custom|FindScene
  (params (NextScene :type Integer))
  (Variables|Default|SetCurrentCameraNumber NextScene)
  (bind _outactors (Actor|GetAllActorsOfClass "/Game/Sample0216/Blueprints/CameraSceneBP.CameraSceneBP_C"))
  (for _array_element _outactors
    (if (== (Variables|/Game/Sample0216/Blueprints/CameraSceneBP.CameraSceneBP_C|GetCameraNumber _array_element) (Variables|Default|GetCurrentCameraNumber)) ; SceneNumberと同じBPを探す
      (Default|ApplyScene _array_element)
      (Default|SetSceneName (Variables|Default|GetSampleWidget) (Variables|/Game/Sample0216/Blueprints/CameraSceneBP.CameraSceneBP_C|GetCameraName _array_element)))))

(event Custom|FindPhoto
  (params (Number :type Integer) (Show :type Boolean))
  (bind _outactors (Actor|GetAllActorsOfClass "/Game/Sample0216/Blueprints/PhotoPlayBP.PhotoPlayBP_C"))
  (for _array_element _outactors
    (if (== (Variables|/Game/Sample0216/Blueprints/PhotoPlayBP.PhotoPlayBP_C|GetNumber _array_element) Number) ; SceneNumberと同じBPを探す
      (Default|PlayPhoto _array_element Show))))

(event EventBeginPlay
  (CallFunction|CreateHUD)
  (CallFunction|SetUp))

(event EventTick
  (params (DeltaSeconds :type Float%20%28single-precision%29))
  (if (Variables|input|GetIsDrag) ; Is Dragging?
    (bind _returnvalue (Class|WidgetLayoutLibrary|GetMousePositiononViewport))
    (switch int (Variables|Default|GetCurrentCameraNumber) ; 2=orbit
      (:1
        (CallFunction|UpdateTurn (.X (Math|Vector2D|BreakVector2D (- _returnvalue (Variables|input|GetStartMousePosition)))) (.Y (Math|Vector2D|BreakVector2D (- _returnvalue (Variables|input|GetStartMousePosition))))))
      (:2
        (if (Variables|Default|GetOrbitInitialized)
          (CallFunction|UpdateOrbit (.X (Math|Vector2D|BreakVector2D (- _returnvalue (Variables|input|GetStartMousePosition)))) (.Y (Math|Vector2D|BreakVector2D (- _returnvalue (Variables|input|GetStartMousePosition)))) (Class|Actor|GetInputAxisKeyValue))
          (else
            (CallFunction|InitOrbit)
            (Variables|Default|SetOrbitInitialized true)))))))

(event Input|MouseEvents|MouseWheelAxis
  (params (AxisValue :type Float%20%28single-precision%29))
  (CallFunction|UpdateOrbit 0.0 0.0 AxisValue))

(event Input|MouseEvents|LeftMouseButton
  (params (Key :type Key%20Structure :default "None"))
  (:Pressed
    (Variables|input|SetIsDrag true)
    (bind _returnvalue (Class|WidgetLayoutLibrary|GetMousePositiononViewport))
    (Variables|input|SetStartMousePosition _returnvalue))
  (:Released
    (Variables|input|SetIsDrag false)))

(fn ConstructionScript)

(fn ChangeCamera
  (params (Mode :type Integer))
  (bind _returnvalue (Game|GetPlayerController 0))
  (bind _blendtime (Variables|Scene|GetBlendTime))
  (bind _output_get (Variables|Default|SetCurrentCameraNumber Mode))
  (switch int _output_get
    (:0
      (Game|Player|SetViewTargetwithBlend _returnvalue _returnvalue _blendtime "VTBlend_Cubic" 0.0 false)
      (Variables|Default|SetCurrentCameraName "Walk"))
    (:1
      (Game|Player|SetViewTargetwithBlend _returnvalue (Variables|Scene|GetTurnCameraActor) _blendtime "VTBlend_Cubic" 0.0 false)
      (Variables|Default|SetCurrentCameraName "Turn"))
    (:2
      (Game|Player|SetViewTargetwithBlend _returnvalue (Variables|Scene|GetOrbitCameraActor) _blendtime "VTBlend_Cubic" 0.0 false)
      (Variables|Default|SetCurrentCameraName "Orbit"))))

(fn UpdateOrbit
  (params (x :type Float%20%28double-precision%29) (y :type Float%20%28double-precision%29) (wheel :type Float%20%28double-precision%29))
  (bind _boostmouse (Variables|Scene|GetBoostMouse))
  (if (Variables|Default|GetOrbitInitialized)
    (Transformation|SetActorRotation (Variables|Scene|GetOrbitCameraActor) (Math|Rotator|MakeRotator (.Roll (Math|Rotator|BreakRotator (Variables|Default|GetOrbitDirection))) (+ (.Pitch (Math|Rotator|BreakRotator (Variables|Default|GetOrbitDirection))) (/ y _boostmouse)) (+ (.Yaw (Math|Rotator|BreakRotator (Variables|Default|GetOrbitDirection))) (* (/ x _boostmouse) -1.0))))
    (Variables|Default|SetOrbitDirection (Math|Rotator|MakeRotator (.Roll (Math|Rotator|BreakRotator (Variables|Default|GetOrbitDirection))) (+ (.Pitch (Math|Rotator|BreakRotator (Variables|Default|GetOrbitDirection))) (/ y _boostmouse)) (+ (.Yaw (Math|Rotator|BreakRotator (Variables|Default|GetOrbitDirection))) (* (/ x _boostmouse) -1.0))))
    (Variables|Default|SetOrbitDistance (+ (* wheel (Variables|Scene|GetBoostWheel)) (Variables|Default|GetOrbitDistance)))
    (Transformation|SetActorLocation (Variables|Scene|GetOrbitCameraActor) (+ (* (Math|Vector|GetForwardVector (Variables|Default|GetOrbitDirection)) (* (Variables|Default|GetOrbitDistance) -1.0)) (Transformation|GetActorLocation (Variables|Scene|GetOrbitTargetActor))) false false)))

(fn UpdateTurn
  (params (x :type Float%20%28double-precision%29) (y :type Float%20%28double-precision%29))
  (bind _returnvalue (Transformation|GetActorRotation))
  (bind _boostmouse (Variables|Scene|GetBoostMouse))
  (bind (_roll _pitch _yaw) (Math|Rotator|BreakRotator _returnvalue))
  (Transformation|SetActorRotation (Variables|Scene|GetTurnCameraActor) (Math|Rotator|MakeRotator _roll (+ _pitch (* (/ y _boostmouse) -1.0)) (+ _yaw (/ x _boostmouse)))))

(fn InitOrbit
  (bind _orbitcameraactor (Variables|Scene|GetOrbitCameraActor))
  (bind _orbittargetactor (Variables|Scene|GetOrbitTargetActor))
  (bind _returnvalue (Transformation|GetActorLocation _orbitcameraactor))
  (bind _returnvalue_2 (Transformation|GetActorLocation _orbittargetactor))
  (Variables|Default|SetOrbitDirection (Math|Rotator|FindLookatRotation _returnvalue _returnvalue_2))
  (Variables|Default|SetOrbitDistance (Math|Vector|VectorLength (- _returnvalue _returnvalue_2))))