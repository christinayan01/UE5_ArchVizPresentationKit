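; Scene marker actor that blends the player or their camera toward its own transform, apparently as a prototype with debug prints.
; GoScene captures the player's start transform at zero Percentage, then lerps the character to this actor by that value.
; ButtonDownEvent1, filtered by MyKind, runs a timeline blending the SampleCharacterBP camera toward a hard-coded position and this actor's rotation.
; Its binding to the GameInstance widget's dispatcher is disconnected.
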(event `self.ReceiveBeginPlay`)

(event `ButtonDownEvent1`
  (params (kind :type Integer))
  (bind _returnvalue (`GameplayStatics.GetPlayerCharacter` 0))
  (`KismetSystemLibrary.PrintString` "Hello")
  (if (== kind (`self.MyKind`))
    (`KismetSystemLibrary.PrintString` "event start")
    (set `self.StartPosition` (`self.K2_GetActorLocation` _returnvalue))
    (set `self.StartRotation` (`self.K2_GetActorRotation` _returnvalue))
    (bind _assample_character_bp (cast `/Game/Sample0216/Blueprints/SampleCharacterBP` _returnvalue))
    (bind (_direction _track) (`Timeline|タイムライン` :!via `PlayFromStart`)
      (:`Update`
        (`KismetSystemLibrary.PrintString` (`KismetStringLibrary.Conv_DoubleToString` _track))
        (`SceneComponent.K2_SetWorldLocationAndRotation` (`/Game/Sample0216/Blueprints/SampleCharacterBP.Camera` _assample_character_bp) (`KismetMathLibrary.VLerp` (`self.StartPosition`) (0.0 4000.0 1500.0) _track) (`KismetMathLibrary.MakeRotator` (`KismetMathLibrary.Lerp` (.roll (`self.StartRotation`)) (.roll (`self.K2_GetActorRotation`)) _track) (`KismetMathLibrary.Lerp` (.pitch (`self.StartRotation`)) (.pitch (`self.K2_GetActorRotation`)) _track) (`KismetMathLibrary.Lerp` 0.0 (.yaw (`self.K2_GetActorRotation`)) _track)) false false))
      (:`Finished`
        (`KismetSystemLibrary.PrintString` "move end")))))

(fn `GoScene`
  (params (percentage :type "Float (double-precision)"))
  (bind _returnvalue (`GameplayStatics.GetPlayerCharacter` 0))
  (bind _returnvalue_2 (`GameplayStatics.GetPlayerCharacter` 0))
  (bind _rootcomponent (`Actor.RootComponent` _returnvalue_2))
  (if (== percentage 0.0)
    (set `self.StartPosition` (`self.K2_GetActorLocation` _returnvalue))
    (set `self.StartRotation` (`self.K2_GetActorRotation` _returnvalue))
    (set `self.EndRotation` (`self.K2_GetActorRotation`)))
  (cast `/Game/Sample0216/Blueprints/SampleCharacterBP` _returnvalue)
  (`SceneComponent.K2_SetWorldLocation` _rootcomponent (`KismetMathLibrary.VLerp` (`self.StartPosition`) (`self.K2_GetActorLocation`) percentage) false false)
  (`SceneComponent.K2_SetWorldRotation` _rootcomponent (`KismetMathLibrary.MakeRotator` (`KismetMathLibrary.Lerp` (.roll (`self.StartRotation`)) (.roll (`self.K2_GetActorRotation`)) percentage) (`KismetMathLibrary.Lerp` (.pitch (`self.StartRotation`)) (.pitch (`self.K2_GetActorRotation`)) percentage) (`KismetMathLibrary.Lerp` (.yaw (`self.StartRotation`)) (.yaw (`self.K2_GetActorRotation`)) percentage)) false false)
  (`KismetSystemLibrary.PrintString` (`KismetSystemLibrary.GetDisplayName` _returnvalue_2)))

(fn `UserConstructionScript`)