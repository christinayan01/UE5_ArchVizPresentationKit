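; CameraSceneBP is a named camera scene that can become the player's active view.
; On BeginPlay it falls back to its own display name if CameraName is empty.
; The ApplyScene event makes it the view target of player controller 0, using a cubic blend over its BlendTime.
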(event `self.ReceiveBeginPlay`
  (if (== (`KismetStringLibrary.Len` (`self.CameraName`)) 0)
    (set `self.CameraName` (`KismetSystemLibrary.GetDisplayName` self))))

(event `ApplyScene`
  (`PlayerController.SetViewTargetWithBlend` (`GameplayStatics.GetPlayerController` 0) self (`self.BlendTime`) "VTBlend_Cubic" 0.0 false))

(fn `UserConstructionScript`)