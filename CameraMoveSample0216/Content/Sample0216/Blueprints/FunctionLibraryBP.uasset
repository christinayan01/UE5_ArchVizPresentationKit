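; Blueprint function library of global getters for the sample's game instance, player controller and game mode, each returned already cast to its project class.
; The player controller getter prefers the reference held by the game mode and falls back to casting player controller 0 when that reference is invalid.
; A failed cast prints an error string naming the getter that failed.
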(fn `GatGameInstanceBP`
  (returns (GameInstance :type "/Game/Sample0216/Blueprints/SampleGameInstance Object Reference"))
  (bind _assample_game_instance (cast `/Game/Sample0216/Blueprints/SampleGameInstance` (`GameplayStatics.GetGameInstance` null))
    (:`then`
      _)
    (:`CastFailed`
      (`KismetSystemLibrary.PrintString` null "ERROR: GetGameInstance")))
  (return _assample_game_instance))

(fn `GetGameModeBP`
  (returns (GameMode :type "/Game/Sample0216/Blueprints/SampleGameModeBP Object Reference"))
  (bind _assample_game_mode_bp (cast `/Game/Sample0216/Blueprints/SampleGameModeBP` (`GameplayStatics.GetGameMode` null))
    (:`then`
      _)
    (:`CastFailed`
      (`KismetSystemLibrary.PrintString` null "ERROR: GetGameMode")))
  (return _assample_game_mode_bp))

(fn `GetPlayerControllerBP`
  (returns (PlayerController :type "/Game/Sample0216/Blueprints/SampleControllerBP Object Reference"))
  (if (`KismetSystemLibrary.IsValid` (`/Game/Sample0216/Blueprints/SampleGameModeBP.PlayerController` (`self.GetGameModeBP` null)))
    (return (`/Game/Sample0216/Blueprints/SampleGameModeBP.PlayerController` (`self.GetGameModeBP` null)))
    (else
      (bind _assample_controller_bp (cast `/Game/Sample0216/Blueprints/SampleControllerBP` (`GameplayStatics.GetPlayerController` null))
        (:`then`
          _)
        (:`CastFailed`
          (`KismetSystemLibrary.PrintString` null "ERROR: GetPlayerController")))
      (return _assample_controller_bp))))