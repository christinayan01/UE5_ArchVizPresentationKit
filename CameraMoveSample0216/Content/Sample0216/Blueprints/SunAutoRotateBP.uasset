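; Day-night cycle controller that advances a SunPosition clock by Multiple seconds per Tick while enabled and shows the time on the player controller's widget.
; A cosine of the time of day serves as sun height, peaking at noon.
; That height scales directional light and skylight intensity, fog and sky sphere color brightness from values cached at BeginPlay, with clamped limits.
; Its normalized form blends post-process white balance temperature.
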(event `self.ReceiveBeginPlay`
  (bind _directionallight (`self.DirectionalLight`))
  (bind _fog (`self.Fog`))
  (bind _skysphere (`self.SkySphere`))
  (bind _skylight (`self.SkyLight`))
  (`|ExecutionSequence`
    (:`then_0`
      (`/Engine/EditorBlueprintResources/StandardMacros.IsValid` _directionallight
        (:`Is Valid`
          (set `self.OriginalSunIntensity` (`LightComponentBase.Intensity` (`Light.LightComponent` _directionallight))))))
    (:`then_1`
      (`/Engine/EditorBlueprintResources/StandardMacros.IsValid` _skylight
        (:`Is Valid`
          (set `self.OriginalSkyIntensity` (`LightComponentBase.Intensity` (`SkyLight.LightComponent` _skylight))))))
    (:`then_2`
      (`/Engine/EditorBlueprintResources/StandardMacros.IsValid` _fog
        (:`Is Valid`
          (set `self.OriginalFogColor` (`ExponentialHeightFogComponent.FogInscatteringLuminance` (`ExponentialHeightFog.Component` _fog))))))
    (:`then_3`
      (set `self.SkyInitZenithColor` (`/Engine/EngineSky/BP_Sky_Sphere.Zenith Color` _skysphere))
      (set `self.SkyInitCloudColor` (`/Engine/EngineSky/BP_Sky_Sphere.Cloud color` _skysphere))
      (set `self.SkyInitOverallColor` (`/Engine/EngineSky/BP_Sky_Sphere.Overall Color` _skysphere))
      (set `self.SkyInitHorizonColor` (`/Engine/EngineSky/BP_Sky_Sphere.Horizon color` _skysphere)))))

(event `UpdateSkySphere`
  (bind _skysphere (`self.SkySphere`))
  (`/Engine/EditorBlueprintResources/StandardMacros.IsValid` _skysphere
    (:`Is Valid`
      (`/Engine/EngineSky/BP_Sky_Sphere.RefreshMaterial` _skysphere))
    (:`Is Not Valid`
      (`KismetSystemLibrary.PrintString` "WARNING: SkySphere is not valid."))))

(event `UpdateSun`
  (bind _originalsunintensity (`self.OriginalSunIntensity`))
  (`/Engine/EditorBlueprintResources/StandardMacros.IsValid` (`self.DirectionalLight`)
    (:`Is Valid`
      (`LightComponent.SetIntensity` (`Light.LightComponent` (`self.DirectionalLight`)) (`KismetMathLibrary.FClamp` (* (`self.GetSunHeight`) _originalsunintensity) (`self.MinValue`) _originalsunintensity)))
    (:`Is Not Valid`
      (`KismetSystemLibrary.PrintString` "WARNING: DirectionalLight is not valid."))))

(event `UpdateSkyLight`
  (bind _originalskyintensity (`self.OriginalSkyIntensity`))
  (`/Engine/EditorBlueprintResources/StandardMacros.IsValid` (`self.SkyLight`)
    (:`Is Valid`
      (`SkyLightComponent.SetIntensity` (`SkyLight.LightComponent` (`self.SkyLight`)) (`KismetMathLibrary.FClamp` (* (`self.GetSunHeight`) _originalskyintensity) (`self.SkyLightMinValue`) _originalskyintensity)))))

(event `UpdateWidgetTime`
  (bind _sunposition (`self.SunPosition`))
  (bind _samplewidget (`/Game/Sample0216/Blueprints/SampleControllerBP.SampleWidget` (`/Game/Sample0216/Blueprints/FunctionLibraryBP.GetPlayerControllerBP`)))
  (`/Engine/EditorBlueprintResources/StandardMacros.IsValid` _sunposition
    (:`Is Valid`
      (`/Game/Sample0216/UI/SampleWidgetBP.setSecond` _samplewidget (`/SunPosition/BP_SunPosition.Seconds` _sunposition))
      (`/Game/Sample0216/UI/SampleWidgetBP.setMinute` _samplewidget (`/SunPosition/BP_SunPosition.Minutes` _sunposition))
      (`/Game/Sample0216/UI/SampleWidgetBP.setHour` _samplewidget (`/SunPosition/BP_SunPosition.Hours` _sunposition)))
    (:`Is Not Valid`
      (`KismetSystemLibrary.PrintString` "WARNING: SunPosition is not valid."))))

(event `UpdateFog`
  (bind (_h _s _v _a) (`KismetMathLibrary.RGBToHSV` (`self.OriginalFogColor`)))
  (`ExponentialHeightFogComponent.SetFogInscatteringColor` (`ExponentialHeightFog.Component` (`self.Fog`)) (`KismetMathLibrary.HSVToRGB` _h _s (`KismetMathLibrary.FClamp` (* _v (`self.GetSunHeight`)) 0.1) _a)))

(event `self.ReceiveTick`
  (params (DeltaSeconds :type "Float (single-precision)"))
  (if (`self.Enable`)
    (`self.UpdateSkySphere`)
    (`self.UpdateSun`)
    (`self.UpdateSkyLight`)
    (`self.UpdateWidgetTime`)
    (`self.UpdateSunPosition`)
    (`self.UpdateWhiteBalance`)
    (`self.UpdateFog`)))

(event `UpdateSunPosition`
  (bind _height (`self.GetSunHeight`))
  (bind _sunposition (`self.SunPosition`))
  (bind _minvalue (`self.MinValue`))
  (bind _skysphere (`self.SkySphere`))
  (bind (_h _s _v _a) (`KismetMathLibrary.RGBToHSV` (`self.SkyInitHorizonColor`)))
  (bind (_h_2 _s_2 _v_2 _a_2) (`KismetMathLibrary.RGBToHSV` (`self.SkyInitZenithColor`)))
  (bind (_h_3 _s_3 _v_3 _a_3) (`KismetMathLibrary.RGBToHSV` (`self.SkyInitCloudColor`)))
  (bind (_h_4 _s_4 _v_4 _a_4) (`KismetMathLibrary.RGBToHSV` (`self.SkyInitOverallColor`)))
  (`/Engine/EditorBlueprintResources/StandardMacros.IsValid` (`self.SunPosition`)
    (:`Is Valid`
      (if (< _height _minvalue)
        (set `self.Coef` _minvalue)
        (else
          (set `self.Coef` _height)))
      (set `/Engine/EngineSky/BP_Sky_Sphere.Zenith Color` (`KismetMathLibrary.HSVToRGB` _h_2 _s_2 (* _v_2 (`self.Coef`)) _a_2) _skysphere)
      (set `/Engine/EngineSky/BP_Sky_Sphere.Cloud color` (`KismetMathLibrary.HSVToRGB` _h_3 _s_3 (* _v_3 (`self.Coef`)) _a_3) _skysphere)
      (set `/Engine/EngineSky/BP_Sky_Sphere.Overall Color` (`KismetMathLibrary.HSVToRGB` _h_4 _s_4 (* _v_4 (`self.Coef`)) _a_4) _skysphere)
      (set `/Engine/EngineSky/BP_Sky_Sphere.Horizon color` (`KismetMathLibrary.HSVToRGB` _h _s (* _v (`self.Coef`)) _a) _skysphere)
      (`/SunPosition/BP_SunPosition.UpdateSun` (`self.SunPosition`))
      (bind _output_get (set `/SunPosition/BP_SunPosition.Seconds` (+ (`/SunPosition/BP_SunPosition.Seconds` _sunposition) (`self.multiple`)) _sunposition))
      (if (>= _output_get 60)
        (bind _output_get_2 (set `/SunPosition/BP_SunPosition.Minutes` (+ (/ _output_get 60) (`/SunPosition/BP_SunPosition.Minutes` _sunposition)) _sunposition))
        (set `/SunPosition/BP_SunPosition.Seconds` (mod _output_get 60) _sunposition)
        (if (== _output_get_2 60)
          (set `/SunPosition/BP_SunPosition.Minutes` 0 _sunposition)
          (bind _result (`/Engine/EditorBlueprintResources/StandardMacros.IncrementInt` (`/SunPosition/BP_SunPosition.Hours` _sunposition))
            (:`  `
              (bind _output_get_3 (set `/SunPosition/BP_SunPosition.Hours` _result _sunposition))
              (if (== _output_get_3 24)
                (set `/SunPosition/BP_SunPosition.Hours` 0 _sunposition)))))))
    (:`Is Not Valid`
      (`KismetSystemLibrary.PrintString` "WARNING: SunPosition is not valid."))))

(event `UpdateWhiteBalance`
  (setmembers `PostProcessSettings` :`StructRef` (`PostProcessVolume.Settings` (`self.PostProcessVolume`)) :`WhiteTemp` (`KismetMathLibrary.Lerp` 4000.0 6000.0 (`self.GetSunHeightNormalized`))))

(fn `GetSunHeight`
  (returns (Height :type "Float (double-precision)"))
  (bind _sunposition (`self.SunPosition`))
  (return (`KismetMathLibrary.DegCos` (+ (* (/ (+ (`/SunPosition/BP_SunPosition.Hours` _sunposition) (/ (`/SunPosition/BP_SunPosition.Minutes` _sunposition) 60.0)) 24.0) 360.0) 180.0))))

(fn `GetSunHeightNormalized`
  (returns (Height :type "Float (double-precision)"))
  (bind _sunposition (`self.SunPosition`))
  (return (`KismetMathLibrary.Lerp` 0.0 0.5 (+ (`KismetMathLibrary.DegCos` (+ (* (/ (+ (`/SunPosition/BP_SunPosition.Hours` _sunposition) (/ (`/SunPosition/BP_SunPosition.Minutes` _sunposition) 60.0)) 24.0) 360.0) 180.0)) 1.0))))

(fn `UserConstructionScript`)