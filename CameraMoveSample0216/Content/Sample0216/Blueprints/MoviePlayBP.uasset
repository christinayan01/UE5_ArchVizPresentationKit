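; MoviePlayBP is an actor that shows and hides a static mesh alongside media player playback, apparently as an in-world movie screen.
; The mesh is hidden on BeginPlay.
; The PlayMovie event takes a Show flag: true reveals the mesh and opens the media source on the media player, while false hides the mesh and pauses the player.
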(event `self.ReceiveBeginPlay`
  (`SceneComponent.SetVisibility` (`self.StaticMesh`) false false))

(event `PlayMovie`
  (params (Show :type Boolean))
  (bind _mediaplayer (`self.MediaPlayer`))
  (bind _staticmesh (`self.StaticMesh`))
  (if Show
    (`SceneComponent.SetVisibility` _staticmesh true false)
    (`MediaPlayer.OpenSource` _mediaplayer (`self.MediaSource`))
    (else
      (`SceneComponent.SetVisibility` _staticmesh false false)
      (`MediaPlayer.Pause` _mediaplayer))))

(fn `UserConstructionScript`)